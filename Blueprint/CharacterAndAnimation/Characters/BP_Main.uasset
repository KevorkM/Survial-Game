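; BP_Main, filed under Characters, tracks Hunger and Hydration as survival stats for the game.
; Its UpdateCharacterProperties event adds incoming deltas to each stat and clamps the results between zero and one.
; It then messages the first player controller's HUD, passing the new totals through delta-named parameters and a constant zero for health.
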(event `/Game/Blueprint/CharacterAndAnimation/Characters/BPI_Character.UpdateCharacterProperties`
  (params (`Delta Health` :type "Float (single-precision)") (`Delta Hydration` :type "Float (single-precision)") (`Delta Hunger` :type "Float (single-precision)"))
  (bind _output_get (set `self.Hunger` (`KismetMathLibrary.FClamp` (+ `Delta Hunger` (`self.Hunger`)))))
  (bind _output_get_2 (set `self.Hydration` (`KismetMathLibrary.FClamp` (+ `Delta Hydration` (`self.Hydration`)))))
  (message `/Game/Blueprint/CharacterAndAnimation/Characters/BPI_Character.UpdateCharacterProperties` (`PlayerController.GetHUD` (`GameplayStatics.GetPlayerController` 0)) 0.0 _output_get_2 _output_get))

(fn `UserConstructionScript`)